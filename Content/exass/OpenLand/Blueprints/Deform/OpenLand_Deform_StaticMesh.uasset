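; OpenLand deformer actor that pairs a configurable static mesh with an OpenLandDeformComponent.
; Its construction script assigns the source mesh and copies the actor's brush material, max depth, area size, debug-line and disable settings to the component.
; The event graph holds only disabled stub events, so any deformation behavior comes from the component.
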(event EventBeginPlay)

(event Collision|EventActorBeginOverlap
  (params (OtherActor :type Actor%20Object%20Reference)))

(event EventTick
  (params (DeltaSeconds :type Float%20%28single-precision%29)))

(fn ConstructionScript
  (Components|StaticMesh|SetStaticMesh (Variables|Default|GetStaticMesh) (Variables|UserInput|GetSourceStaticMesh))
  (Variables|/Game/exass/OpenLand/Blueprints/Deform/OpenLand_DeformComponent.OpenLand_DeformComponent_C|SetBrush%20Material (Variables|Default|GetOpenLand_DeformComponent) (Variables|UserInput|GetBrushMaterial))
  (Variables|/Game/exass/OpenLand/Blueprints/Deform/OpenLand_DeformComponent.OpenLand_DeformComponent_C|SetMaxDepth (Variables|Default|GetOpenLand_DeformComponent) (Variables|UserInput|GetMaxDepth))
  (Variables|/Game/exass/OpenLand/Blueprints/Deform/OpenLand_DeformComponent.OpenLand_DeformComponent_C|SetArea%20Size (Variables|Default|GetOpenLand_DeformComponent) (Variables|UserInput|GetAreaSize))
  (Variables|/Game/exass/OpenLand/Blueprints/Deform/OpenLand_DeformComponent.OpenLand_DeformComponent_C|SetDrawDebugLine (Variables|Default|GetOpenLand_DeformComponent) (Variables|UserInput|GetDrawDebugLine))
  (Variables|/Game/exass/OpenLand/Blueprints/Deform/OpenLand_DeformComponent.OpenLand_DeformComponent_C|SetDisable (Variables|Default|GetOpenLand_DeformComponent) (Variables|UserInput|GetDisable)))