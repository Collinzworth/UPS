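; Utility functions for the OpenLand tools that invalidate the Material and Height runtime virtual textures, each behind its own flag.
; Each finds one RVT volume actor per type with GetActorOfClass and, if valid, calls Invalidate on its virtual texture component.
; InvalidateRVTs covers the volume's bounds with a huge sphere radius, while InvalidateRVTsPartial takes an origin and radius but still passes the volume's full box extent.
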(fn InvalidateRVTs
  (params (Use%20MaterialRVT :type Boolean) (Use%20HeightRVT :type Boolean))
  (Utilities|FlowControl|Sequence
    (:then_0
      (if Use%20MaterialRVT
        (bind _returnvalue (Actor|GetActorOfClass 0 "/Game/exass/OpenLand(MustBuyIfUse)/Core/RVT/BP_OpenLand_RVT_Volume_Material.BP_OpenLand_RVT_Volume_Material_C"))
        (Utilities|IsValid _returnvalue
          (:Is%20Valid
            (Class|RuntimeVirtualTextureComponent|Invalidate (Variables|/Script/Engine.RuntimeVirtualTextureVolume|GetVirtualTextureComponent _returnvalue) (Utilities|Struct|MakeBoxSphereBounds (.Origin (Collision|GetActorBounds _returnvalue false false)) (.BoxExtent (Collision|GetActorBounds _returnvalue false false)) 9999999.0))))))
    (:then_1
      (if Use%20HeightRVT
        (bind _returnvalue_2 (Actor|GetActorOfClass 0 "/Game/exass/OpenLand(MustBuyIfUse)/Core/RVT/BP_OpenLand_RVT_Volume_Height.BP_OpenLand_RVT_Volume_Height_C"))
        (Utilities|IsValid _returnvalue_2
          (:Is%20Valid
            (Class|RuntimeVirtualTextureComponent|Invalidate (Variables|/Script/Engine.RuntimeVirtualTextureVolume|GetVirtualTextureComponent _returnvalue_2) (Utilities|Struct|MakeBoxSphereBounds (.Origin (Collision|GetActorBounds _returnvalue_2 false false)) (.BoxExtent (Collision|GetActorBounds _returnvalue_2 false false)) 9999999.0))))))))

(fn InvalidateRVTsPartial
  (params (Use%20MaterialRVT :type Boolean) (Use%20HeightRVT :type Boolean) (Origin :type Vector) (Radius :type Float%20%28double-precision%29))
  (Utilities|FlowControl|Sequence
    (:then_0
      (if Use%20MaterialRVT
        (bind _returnvalue (Actor|GetActorOfClass 0 "/Game/exass/OpenLand(MustBuyIfUse)/Core/RVT/BP_OpenLand_RVT_Volume_Material.BP_OpenLand_RVT_Volume_Material_C"))
        (Utilities|IsValid _returnvalue
          (:Is%20Valid
            (Class|RuntimeVirtualTextureComponent|Invalidate (Variables|/Script/Engine.RuntimeVirtualTextureVolume|GetVirtualTextureComponent _returnvalue) (Utilities|Struct|MakeBoxSphereBounds Origin (.BoxExtent (Collision|GetActorBounds _returnvalue false false)) Radius))))))
    (:then_1
      (if Use%20HeightRVT
        (bind _returnvalue_2 (Actor|GetActorOfClass 0 "/Game/exass/OpenLand(MustBuyIfUse)/Core/RVT/BP_OpenLand_RVT_Volume_Height.BP_OpenLand_RVT_Volume_Height_C"))
        (Utilities|IsValid _returnvalue_2
          (:Is%20Valid
            (Class|RuntimeVirtualTextureComponent|Invalidate (Variables|/Script/Engine.RuntimeVirtualTextureVolume|GetVirtualTextureComponent _returnvalue_2) (Utilities|Struct|MakeBoxSphereBounds Origin (.BoxExtent (Collision|GetActorBounds _returnvalue_2 false false)) Radius))))))))