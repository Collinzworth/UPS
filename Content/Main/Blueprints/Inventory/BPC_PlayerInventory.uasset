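; Player inventory component that extends a parent container with slot drag-and-drop handling and UI updates.
; Slot drops from a Player Inventory container call that source's TransferItem into this component at the dropped index; no other container type is handled.
; Add and remove overrides run the parent logic, then message the owning character's controller to update or reset the affected slot.
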(event EventBeginPlay
  (|CallParentFunction) ; This node is disabled and will not be called.\nDrag off pins to build functionality.
)

(event EventTick
  (params (DeltaSeconds :type Float%20%28single-precision%29))
  (|CallParentFunction DeltaSeconds) ; This node is disabled and will not be called.\nDrag off pins to build functionality.
)

(fn HandleSlotDrop
  (params (FromContainer :type BPC%20Items%20Container%20Object%20Reference) (FromIndex :type Integer) (DroppedIndex :type Integer))
  (LocalVariables|SetLocalFromContainer FromContainer)
  (LocalVariables|SetLocalFromIndes FromIndex)
  (LocalVariables|SetLocalDropIndex DroppedIndex)
  (switch Utilities|FlowControl|Switch|SwitchonE_ContainerType (Variables|/Game/Main/Blueprints/Inventory/BPC_ItemsContainer.BPC_ItemsContainer_C|GetContainerType (LocalVariables|GetLocalFromContainer))
    (:NewEnumerator0
      (Default|TransferItem (LocalVariables|GetLocalFromContainer) self (LocalVariables|GetLocalDropIndex) (LocalVariables|GetLocalFromIndes))
      (return))))

(fn AddItemtoIndex
  (params (Item :type S%20Item%20Info%20Structure) (LocalSpecificIndex :type Integer) (FromIndex :type Integer))
  ;[1 0.8659 0] UI-Related
  (bind _success (|CallParentFunction Item LocalSpecificIndex FromIndex))
  (bind _controllerref (Class|BPISurvivalCharacter|GetControllerfromChar(Message) (Components|GetOwner)))
  (Default|UpdateItemSlot _controllerref (Variables|Default|GetContainerType) LocalSpecificIndex (CallFunction|GetItematIndex LocalSpecificIndex))
  (return _success))

(fn RemoveItematIndex
  (params (Index :type Integer))
  ;[1 0.8487 0] UI-Related
  (bind _success_ (|CallParentFunction Index))
  (bind _controllerref (Class|BPISurvivalCharacter|GetControllerfromChar(Message) (Components|GetOwner)))
  (Default|ResetItemSlot _controllerref (Variables|Default|GetContainerType) Index)
  (return _success_))